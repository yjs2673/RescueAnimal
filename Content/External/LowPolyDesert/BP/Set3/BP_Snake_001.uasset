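; BP_Snake_001 is a snake actor from the LowPolyDesert set with separately tintable body, eyes and bottom.
; Its construction script creates a dynamic material instance on the first material slot of the Snake, Eyes and Bottom components.
; Each instance gets its ColorParameter set from that part's color value.
; The event graph holds only disabled placeholder events, so the asset has no runtime logic.
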(event EventBeginPlay)

(event Collision|EventActorBeginOverlap
  (params (OtherActor :type Actor%20Object%20Reference)))

(event EventTick
  (params (DeltaSeconds :type Float%20%28single-precision%29)))

(fn ConstructionScript
  (bind _returnvalue (Rendering|Material|CreateDynamicMaterialInstance (Variables|Default|GetSnake) 0 0 "None" :!class /Script/Engine.PrimitiveComponent))
  (Rendering|Material|SetVectorParameterValue _returnvalue "ColorParameter" (Variables|Colors|GetSnake_) :!class /Script/Engine.MaterialInstanceDynamic)
  (bind _returnvalue_2 (Rendering|Material|CreateDynamicMaterialInstance (Variables|Default|GetEyes) 0 0 "None" :!class /Script/Engine.PrimitiveComponent))
  (Rendering|Material|SetVectorParameterValue _returnvalue_2 "ColorParameter" (Variables|Colors|GetEyes_) :!class /Script/Engine.MaterialInstanceDynamic)
  (bind _returnvalue_3 (Rendering|Material|CreateDynamicMaterialInstance (Variables|Default|GetBottom) 0 0 "None" :!class /Script/Engine.PrimitiveComponent))
  (Rendering|Material|SetVectorParameterValue _returnvalue_3 "ColorParameter" (Variables|Colors|GetBottom_) :!class /Script/Engine.MaterialInstanceDynamic))